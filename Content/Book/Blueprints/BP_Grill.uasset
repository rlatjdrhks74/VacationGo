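; BP_Grill is a possessable grill pawn that the player character can enter, and which leads to the GameplayC level.
; Its box overlap sets or clears the Grill reference on BP_VGCharacter, with registration allowed only while no player controller possesses it.
; Pressing GetBoat while possessed calls OpenLevel for GameplayC, then spawns a new character beside the grill, hands possession to it and spawns a default controller.
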(event `self.Box.OnComponentBeginOverlap`
  (params (OverlappedComponent :type "PrimitiveComponent Object Reference") (OtherActor :type "Actor Object Reference") (OtherComp :type "PrimitiveComponent Object Reference") (OtherBodyIndex :type Integer) (bFromSweep :type Boolean) (SweepResult :type "HitResult Structure (by ref)"))
  (if (`self.Can be entered`)
    (bind _asbp_vgcharacter (cast `/Game/Book/Blueprints/BP_VGCharacter` OtherActor))
    (set `/Game/Book/Blueprints/BP_VGCharacter.Grill` self _asbp_vgcharacter)))

(event `self.Box.OnComponentEndOverlap`
  (params (OverlappedComponent :type "PrimitiveComponent Object Reference") (OtherActor :type "Actor Object Reference") (OtherComp :type "PrimitiveComponent Object Reference") (OtherBodyIndex :type Integer))
  (bind _asbp_vgcharacter (cast `/Game/Book/Blueprints/BP_VGCharacter` OtherActor))
  (if (== self (`/Game/Book/Blueprints/BP_VGCharacter.Grill` _asbp_vgcharacter))
    (set `/Game/Book/Blueprints/BP_VGCharacter.Grill` null _asbp_vgcharacter)))

(event `self.ReceivePossessed`
  (params (NewController :type "Controller Object Reference"))
  (cast `PlayerController` NewController)
  (set `self.Can be entered` false))

(event `self.ReceiveUnpossessed`
  (params (OldController :type "Controller Object Reference"))
  (cast `PlayerController` OldController)
  (set `self.Can be entered` true))

(event `InputAction|GetBoat`
  (params (Key :type "Key Structure"))
  (bind _defaultsceneroot (`self.DefaultSceneRoot`))
  (bind (_relativerotation_roll _relativerotation_pitch _relativerotation_yaw) (`KismetMathLibrary.BreakRotator` (`SceneComponent.RelativeRotation` _defaultsceneroot)))
  (:`Pressed`
    (`GameplayStatics.OpenLevel` "GameplayC")
    (bind _returnvalue (`|SpawnActorFromClass` "/Game/Book/Blueprints/BP_VGCharacter.BP_VGCharacter_C" (`KismetMathLibrary.Conv_VectorToTransform` (+ (`SceneComponent.K2_GetComponentLocation` _defaultsceneroot) (* (`KismetMathLibrary.GetRightVector` (`KismetMathLibrary.MakeRotator` _relativerotation_roll _relativerotation_pitch _relativerotation_yaw)) -200.0) (0.0 0.0 125.0))) "AlwaysSpawn" "OverrideRootScale" null null))
    (`Controller.Possess` (`self.GetController`) _returnvalue)
    (`self.SpawnDefaultController`)))

(fn `UserConstructionScript`)